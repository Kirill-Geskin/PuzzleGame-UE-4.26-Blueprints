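; Puzzle character Blueprint that can jump and carries a selection cursor widget component to show when it is selected.
; EnableSelectWidget shows the cursor and plays its SelectWidget animation on an endless loop, while DisableSelectWidget stops the animation and hides it.
; The cursor starts disabled on BeginPlay; nothing in this Blueprint enables it, and Jump input triggers the standard jump.
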(event `self.ReceiveBeginPlay`
  (`self.DisableSelectWidget`))

(event `InputAction|Jump`
  (params (Key :type "Key Structure"))
  (:`Pressed`
    (`self.Jump`)))

(fn `DisableSelectWidget`
  (bind _selectioncursor (`self.SelectionCursor`))
  (bind _asselect_widget (cast `/Game/HUD/SelectWidget` (`WidgetComponent.GetUserWidgetObject` _selectioncursor)))
  (`UserWidget.StopAnimation` _asselect_widget (`/Game/HUD/SelectWidget.CursorAnimation` _asselect_widget))
  (`SceneComponent.SetVisibility` _selectioncursor false false))

(fn `EnableSelectWidget`
  (bind _selectioncursor (`self.SelectionCursor`))
  (bind _returnvalue (`WidgetComponent.GetUserWidgetObject` _selectioncursor))
  (bind _asselect_widget (cast `/Game/HUD/SelectWidget` _returnvalue))
  (`UserWidget.PlayAnimation` _returnvalue (`/Game/HUD/SelectWidget.CursorAnimation` _asselect_widget) 0.0 0 "Forward" 1.0 false)
  (`SceneComponent.SetVisibility` _selectioncursor true false))

(fn `UserConstructionScript`)